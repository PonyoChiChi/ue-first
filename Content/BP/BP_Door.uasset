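; BP_Door is an interactable door actor that swings between two yaw angles each time it is interacted with.
; ReactonInteraction flips IsOpened and activates rotation, which Tick applies with FInterpTo at RotationSpeed until yaw nearly equals the target.
; Targets are fixed absolute actor yaws rather than offsets from placement, with IsOpened true selecting zero.
; The construction script assigns TutorialTPP_Mat to the Cube mesh.
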(event EventTick
  (params (DeltaSeconds :type Float%20%28single-precision%29))
  (bind _isopened (Variables|Default|GetIsOpened))
  (bind _returnvalue (Math|Float|SelectFloat 0.0 1e+02 _isopened))
  (Variables|Default|SetDelta%20Seconds DeltaSeconds)
  (if (Variables|Default|GetIsDoorRotationActive)
    (Transformation|SetActorRotation (Math|Rotator|MakeRotator 0.0 0.0 (Math|Interpolation|FInterpTo (.yaw (Transformation|GetActorRotation)) _returnvalue (Variables|Default|GetDelta%20Seconds) (Variables|Default|GetRotationSpeed))))
    (if (Math|Float|NearlyEqual(Float) (Math|Interpolation|FInterpTo (.yaw (Transformation|GetActorRotation)) _returnvalue (Variables|Default|GetDelta%20Seconds) (Variables|Default|GetRotationSpeed)) _returnvalue 1e-06)
      (Variables|Default|SetIsDoorRotationActive false))))

(event EventReactonInteraction
  (Variables|Default|SetIsDoorRotationActive true)
  (Variables|Default|SetIsOpened (not (Variables|Default|GetIsOpened))))

(fn ConstructionScript
  (Rendering|Material|SetMaterial (Variables|Default|GetCube) 0 "/Engine/Tutorial/SubEditors/TutorialAssets/Character/TutorialTPP_Mat.TutorialTPP_Mat"))