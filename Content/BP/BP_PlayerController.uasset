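; Player controller that handles first-hand input for mouse look, movement and interaction through Enhanced Input actions.
; Look input drives the pawn's yaw and inverted pitch, while movement follows control-rotation forward and right vectors.
; On interact completion, it line traces from the character's camera, fetched by message call, with debug drawing.
; Hit actors tagged "interactable" receive a reaction message, keeping interaction logic in the target.
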(event Input|EnhancedActionEvents|EnhancedInputActionIA_InputAction
  (params (ActionValue :type Vector%202D%20Structure) (ElapsedSeconds :type Float%20%28double-precision%29) (TriggeredSeconds :type Float%20%28double-precision%29) (InputAction :type Input%20Action%20Object%20Reference :default "/Game/Input/IA_InputAction.IA_InputAction"))
  (bind _returnvalue (Pawn|GetControlRotation :!class /Script/Engine.Controller))
  ;[1 1 1] Movement
  (Pawn|Input|AddMovementInput (Game|Player|GetPlayerPawn 0) (Math|Vector|GetRightVector (Math|Rotator|MakeRotator (.roll _returnvalue) 0.0 (.yaw _returnvalue))) (.y ActionValue) false)
  (Pawn|Input|AddMovementInput (Game|Player|GetPlayerPawn 0) (Math|Vector|GetForwardVector (Math|Rotator|MakeRotator 0.0 0.0 (.yaw (Pawn|GetControlRotation :!class /Script/Engine.Controller)))) (.x ActionValue) false))

(event Input|EnhancedActionEvents|EnhancedInputActionIA_Interact
  (params (ActionValue :type Boolean) (ElapsedSeconds :type Float%20%28double-precision%29) (TriggeredSeconds :type Float%20%28double-precision%29) (InputAction :type Input%20Action%20Object%20Reference :default "/Game/Input/IA_Interact.IA_Interact"))
  ;[1 1 1] Interact
  (:Completed
    (bind _playercamera (Class|BPInteractInterface|GetPlayerCamera(Message) (Game|GetPlayerCharacter 0)))
    (bind (_outhit _returnvalue) (Collision|LineTraceByChannel (Transformation|GetWorldLocation _playercamera) (+ (Transformation|GetWorldLocation _playercamera) (* (Math|Vector|GetForwardVector _playercamera) (Variables|Default|GetInteractionDistance))) "TraceTypeQuery1" false 0 "ForDuration"))
    (if _returnvalue
      (if (and (Actor|ActorHasTag (.HitActor (Collision|BreakHitResult _outhit)) "interactable") (Utilities|IsValid (.HitActor (Collision|BreakHitResult _outhit))))
        (Class|BPInteractionObjectInterface|ReactonInteraction(Message) (.HitActor (Collision|BreakHitResult _outhit)))))))

(event Input|EnhancedActionEvents|EnhancedInputActionIA_MouseLook
  (params (ActionValue :type Vector%202D%20Structure) (ElapsedSeconds :type Float%20%28double-precision%29) (TriggeredSeconds :type Float%20%28double-precision%29) (InputAction :type Input%20Action%20Object%20Reference :default "/Game/Input/IA_MouseLook.IA_MouseLook"))
  ;[1 1 1] Mouse look
  (Pawn|Input|AddControllerYawInput (Game|Player|GetPlayerPawn 0) (.x ActionValue))
  (Pawn|Input|AddControllerPitchInput (Game|Player|GetPlayerPawn 0) (* (.y ActionValue) -1.0)))

(fn ConstructionScript)